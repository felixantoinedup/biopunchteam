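; BP_FloorTile is a track segment for an endless runner that spawns a random obstacle and recycles the track.
; Its construction script gathers three spawn point transforms and adds a blocker child actor at a random one.
; When the RunCharacter overlaps EndTrigger, it asks the game mode to add another tile, then destroys itself after a short delay.
; GetAttachTransform exposes the AttachPoint world transform.
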(event `self.EndTrigger.OnComponentBeginOverlap`
  (params (OverlappedComponent :type "PrimitiveComponent Object Reference") (OtherActor :type "Actor Object Reference") (OtherComp :type "PrimitiveComponent Object Reference") (OtherBodyIndex :type Integer) (bFromSweep :type Boolean) (SweepResult :type "HitResult Structure (by ref)"))
  (cast `/Game/Tuto/EndlessRunner/RunCharacter` OtherActor)
  (bind _asendless_runner_game_mode (cast `/Game/Tuto/EndlessRunner/EndlessRunnerGameMode` (`GameplayStatics.GetGameMode`)))
  (`/Game/Tuto/EndlessRunner/EndlessRunnerGameMode.AddFloorTile` _asendless_runner_game_mode)
  (`KismetSystemLibrary.Delay` 2.0)
  (`self.K2_DestroyActor`))

(fn `GetAttachTransform`
  (returns (AttachTransform :type "Transform Structure"))
  (return (`SceneComponent.K2_GetComponentToWorld` (`self.AttachPoint`))))

(fn `SetSpawnPoints`
  (set `self.SpawnPoints` (`|MakeArray` (`SceneComponent.GetRelativeTransform` (`self.SpawnPoint1`)) (`SceneComponent.GetRelativeTransform` (`self.SpawnPoint2`)) (`SceneComponent.GetRelativeTransform` (`self.SpawnPoint3`)))))

(fn `SpawnBlocker`
  (bind _spawnpoints (`self.SpawnPoints`))
  (`AddComponent|NODE_AddChildActorComponent-0` :`RelativeTransform` (`|GetArrayItem` _spawnpoints (`KismetMathLibrary.RandomIntegerInRange` 0 (`KismetArrayLibrary.Array_LastIndex` _spawnpoints)))))

(fn `UserConstructionScript`
  (`self.SetSpawnPoints`)
  (`self.SpawnBlocker`))