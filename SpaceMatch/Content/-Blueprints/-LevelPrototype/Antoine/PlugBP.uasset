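; PlugBP is a shape-typed plug that a robot can grab and place, showing its type (square, sphere, cylinder or cone) as text set on BeginPlay.
; Held and placed flags guard GrabPlug and PlacePlug, so a placed plug cannot be grabbed again and placing notifies the holding RobotBP.
; Both share SetPlug, which changes the holder, zeroes velocities, attaches to the given parent and disables physics.
; LaunchPlug is an empty stub.
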(event `self.ReceiveBeginPlay`
  (`self.Set Plug Type Text`))

(event `Set Plug Type Text`
  (switch `/Game/-Blueprints/-LevelPrototype/Antoine/PlugType` (`self.PlugType`)
    (:`NewEnumerator0`
      (set `self.StringType` "Square"))
    (:`NewEnumerator1`
      (set `self.StringType` "Sphere"))
    (:`NewEnumerator2`
      (set `self.StringType` "Cylinder"))
    (:`NewEnumerator3`
      (set `self.StringType` "Cone")))
  (`TextRenderComponent.K2_SetText` (`self.TextType`) (`self.StringType`)))

(fn `GrabPlug`
  (params (NewHolder :type "Actor Object Reference") (Parent :type "SceneComponent Object Reference"))
  (if (`self.IsHolded`)
    _
    (elif (not (`self.IsPlaced`))
      (`self.SetPlug` NewHolder Parent)
      (set `self.IsHolded` true)
      (set `self.IsPlaced` false))))

(fn `LaunchPlug`)

(fn `PlacePlug`
  (params (NewHolder :type "Actor Object Reference") (Parent :type "SceneComponent Object Reference"))
  (if (`self.IsHolded`)
    (bind _asrobot_bp (cast `/Game/-Blueprints/RobotBP` (`self.Holder`)))
    (`/Game/-Blueprints/RobotBP.PlacePlug` _asrobot_bp)
    (`self.SetPlug` NewHolder Parent)
    (set `self.IsHolded` false)
    (set `self.IsPlaced` true)))

(fn `SetPlug`
  (params (NewHolder :type "Actor Object Reference") (Parent :type "SceneComponent Object Reference"))
  (bind _plug (`self.Plug`))
  (set `self.Holder` NewHolder)
  (`PrimitiveComponent.SetPhysicsLinearVelocity` _plug (0.0 0.0 0.0) false "None")
  (`PrimitiveComponent.SetPhysicsAngularVelocityInRadians` _plug (0.0 0.0 0.0) false "None")
  (`self.K2_AttachToComponent` Parent "None" "KeepRelative" "KeepRelative" "KeepRelative")
  (`SceneComponent.K2_SetRelativeLocation` (`self.Plug`) (0.0 0.0 0.0) false false)
  (`PrimitiveComponent.SetSimulatePhysics` (`self.Plug`) false))

(fn `UserConstructionScript`)