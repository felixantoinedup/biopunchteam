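; SocketBP is a puzzle socket that accepts a matching plug carried by an overlapping RobotBP.
; Placement requires the same PlugType, aligned up vectors and, when the socket has arrow components, at least one forward-aligned arrow pair, checked with dot products against RotationTolerance.
; On success, the robot attaches the plug, the socket notifies SectionController and flags wires active, though the per-wire loop is empty.
; BeginPlay labels the socket with its type.
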(event `self.ReceiveBeginPlay`
  (set `self.ArrowComponents` (`self.K2_GetComponentsByClass` "/Script/Engine.ArrowComponent"))
  (switch `/Game/-Blueprints/-LevelPrototype/Antoine/PlugType` (`self.PlugType`)
    (:`NewEnumerator6`
      (set `self.StringType` "Cross"))
    (:`NewEnumerator7`
      (set `self.StringType` "Plain"))
    (:`NewEnumerator8`
      (set `self.StringType` "TShape"))
    (:`NewEnumerator9`
      (set `self.StringType` "UpDiago"))
    (:`NewEnumerator2`
      (set `self.StringType` "UpDown"))
    (:`NewEnumerator4`
      (set `self.StringType` "UpLeft"))
    (:`NewEnumerator0`
      (set `self.StringType` "Up"))
    (:`NewEnumerator10`
      (set `self.StringType` "VShape")))
  (`TextRenderComponent.K2_SetText` (`self.TextType`) (`self.StringType`)))

(event `self.ReceiveActorBeginOverlap`
  (params (OtherActor :type "Actor Object Reference"))
  (bind _arrowcomponents (`self.ArrowComponents`))
  (if (not (`self.HoldingPlug`))
    (bind _asrobot_bp (cast `/Game/-Blueprints/RobotBP` OtherActor))
    (bind _holdedplug (`/Game/-Blueprints/RobotBP.HoldedPlug` _asrobot_bp))
    (if (`|EnumEquality` (`/Game/-Blueprints/-LevelPrototype/Antoine/PlugBP.PlugType` _holdedplug) (`self.PlugType`))
      (if (> (`KismetMathLibrary.Dot_VectorVector` (`SceneComponent.GetUpVector` (`self.DefaultSceneRoot`)) (`SceneComponent.GetUpVector` (`Actor.RootComponent` _holdedplug))) (`self.RotationTolerance`))
        (set `self.CanPlacePlug` false)
        (if (> (`KismetArrayLibrary.Array_Length` _arrowcomponents) 0)
          (for _array_element _arrowcomponents :!label _label
            (for _array_element_2 (`/Game/-Blueprints/-LevelPrototype/Antoine/PlugBP.ArrowComponents` _holdedplug)
              (if (> (`KismetMathLibrary.Dot_VectorVector` (`SceneComponent.GetForwardVector` _array_element_2) (`SceneComponent.GetForwardVector` _array_element)) (`self.RotationTolerance`))
                (set `self.CanPlacePlug` true)
                (goto _label :!via `Break`))))
          (if (`self.CanPlacePlug`)
            (`/Game/-Blueprints/RobotBP.PlacePlug` _asrobot_bp self (`self.PlugPosition`) :!label _label_2)
            (set `self.HoldingPlug` true)
            (`/Game/-Blueprints/-LevelPrototype/Antoine/SectionControllerBP.OnPlugPlaced` (`self.SectionController`) (`self.PlugType`))
            (`self.ActivateWires`))
          (else
            (goto _label_2)))))))

(event `ActivateWires`
  (set `self.WiresAreActive` true)
  (for _ (`self.Wires`)
    _))

(fn `UserConstructionScript`)