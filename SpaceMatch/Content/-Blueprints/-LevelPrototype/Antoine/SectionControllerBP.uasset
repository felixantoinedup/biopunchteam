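; Level section controller for a plug-and-socket puzzle that opens a door and initializes the next section once solved.
; On initialization it builds the required plug list from its sockets and can launch those plugs, plus random extras, inside a spawn area.
; OnPlugPlaced checks off matching types and activates wires in socket order up to the first empty socket.
; When the count runs out, FinishSection also destroys unplaced plugs.
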(event `self.ReceiveBeginPlay`
  (set `self.UsableSectionSockets` (`self.SectionSockets`))
  (if (`self.Initialize At Start`)
    (`self.Initialize Section`)))

(event `Initialize Section`
  (`self.CreateSequence`)
  (for _array_element (`self.SectionSockets`)
    (set `/Game/-Blueprints/-LevelPrototype/Antoine/SocketBP.SectionController` self _array_element))
  (if (`self.SpawnPlugAtInit`)
    (`self.SpawnPlugs`)))

(fn `CreateSequence`
  (locals (RandomIndex :type Integer :default 0))
  (for _array_element (`self.UsableSectionSockets`)
    (bind _result (`/Engine/EditorBlueprintResources/StandardMacros.IncrementInt` (`self.NbrPlugsSequence`))
      (:`  `
        (bind _output_get (set `self.NbrPlugsSequence` _result))
        (set `self.CurrentNbrPlugsSequence` _output_get)
        (`KismetArrayLibrary.Array_Add` (`self.SequecePlugs`) (`/Game/-Blueprints/-LevelPrototype/Antoine/SocketBP.PlugType` _array_element))
        (`KismetArrayLibrary.Array_Add` (`self.SequencePlugsChecks`)))))
  (`KismetArrayLibrary.Array_Clear` (`self.UsableSectionSockets`)))

(fn `DespawnPlugs`
  (bind _plugssection (`self.PlugsSection`))
  (for (_ _array_index) _plugssection
    (bind _output (`|GetArrayItem` _plugssection _array_index))
    (if (not (`/Game/-Blueprints/-LevelPrototype/Antoine/PlugBP.IsPlaced` _output))
      (`self.K2_DestroyActor` _output))))

(fn `FinishSection`
  (`self.Initialize Section` (`self.NextSectionController`))
  (`/Game/-Blueprints/-LevelPrototype/Antoine/DoorBP.Open Door` (`self.Door`))
  (`self.DespawnPlugs`))

(fn `OnPlugPlaced`
  (params (PlacedPlugType :type "/Game/-Blueprints/-LevelPrototype/Antoine/PlugType Enum" :default "NewEnumerator0"))
  (for (_array_element _array_index) (`self.SequecePlugs`)
    (if (`|EnumEquality` PlacedPlugType _array_element)
      (bind _output (`|GetArrayItem` (`self.SequencePlugsChecks`) _array_index))
      (if (not _output)
        (`|VariableSetRef` _output true)
        (for _array_element_2 (`self.SectionSockets`)
          (if (`/Game/-Blueprints/-LevelPrototype/Antoine/SocketBP.HoldingPlug` _array_element_2)
            (if (not (`/Game/-Blueprints/-LevelPrototype/Antoine/SocketBP.WiresAreActive` _array_element_2))
              (set `/Game/-Blueprints/-LevelPrototype/Antoine/SocketBP.WiresAreActive` true _array_element_2)
              (`/Game/-Blueprints/-LevelPrototype/Antoine/SocketBP.ActivateWires` _array_element_2))
            (else
              (break))))
        (bind _result (`/Engine/EditorBlueprintResources/StandardMacros.DecrementInt` (`self.CurrentNbrPlugsSequence`))
          (:`  `
            (if (< _result 1)
              (`self.FinishSection`)
              (else
                (return)))))))))

(fn `SpawnPlug`
  (params (Transfrom :type "Transform Structure") (PlugType :type "/Game/-Blueprints/-LevelPrototype/Antoine/PlugType Enum" :default "NewEnumerator0"))
  (locals (PlugTypeClass :type "Actor Object Reference" :default "BlueprintGeneratedClass'/Game/-Blueprints/-LevelPrototype/Antoine/PlugBP.PlugBP_C'"))
  (switch `/Game/-Blueprints/-LevelPrototype/Antoine/PlugType` PlugType
    (:`NewEnumerator6`
      (set `local.PlugTypeClass` "/Game/-Blueprints/-LevelPrototype/Antoine/Plugs/CrossPlugBP.CrossPlugBP_C"))
    (:`NewEnumerator7`
      (set `local.PlugTypeClass` "/Game/-Blueprints/-LevelPrototype/Antoine/Plugs/PlainPlugBP.PlainPlugBP_C"))
    (:`NewEnumerator8`
      (set `local.PlugTypeClass` "/Game/-Blueprints/-LevelPrototype/Antoine/Plugs/TShapePlugBP.TShapePlugBP_C"))
    (:`NewEnumerator9`
      (set `local.PlugTypeClass` "/Game/-Blueprints/-LevelPrototype/Antoine/Plugs/UpDiagoPlugBP.UpDiagoPlugBP_C"))
    (:`NewEnumerator2`
      (set `local.PlugTypeClass` "/Game/-Blueprints/-LevelPrototype/Antoine/Plugs/UpDownPlugBP.UpDownPlugBP_C"))
    (:`NewEnumerator4`
      (set `local.PlugTypeClass` "/Game/-Blueprints/-LevelPrototype/Antoine/Plugs/UpLeftPlugBP.UpLeftPlugBP_C"))
    (:`NewEnumerator0`
      (set `local.PlugTypeClass` "/Game/-Blueprints/-LevelPrototype/Antoine/Plugs/UpPlugBP.UpPlugBP_C"))
    (:`NewEnumerator10`
      (set `local.PlugTypeClass` "/Game/-Blueprints/-LevelPrototype/Antoine/Plugs/VShapePlugBP.VShapePlugBP_C")))
  (bind _returnvalue (`|SpawnActorFromClass` (`local.PlugTypeClass`) Transfrom "AdjustIfPossibleButAlwaysSpawn" "OverrideRootScale" null null))
  (bind _asplug_bp (cast `/Game/-Blueprints/-LevelPrototype/Antoine/PlugBP` _returnvalue))
  (set `/Game/-Blueprints/-LevelPrototype/Antoine/PlugBP.PlugType` PlugType _asplug_bp)
  (bind _plug (`/Game/-Blueprints/-LevelPrototype/Antoine/PlugBP.Plug` _asplug_bp))
  (`PrimitiveComponent.AddImpulse` _plug (* (`KismetMathLibrary.RandomUnitVector`) (`KismetMathLibrary.RandomFloatInRange` (`self.PlugSpawnVelocityMin`) (`self.PlugSpawnVelocityMax`))) "None" false)
  (`PrimitiveComponent.AddAngularImpulseInRadians` _plug (* (`KismetMathLibrary.RandomUnitVector`) (`KismetMathLibrary.RandomFloatInRange` (`self.PlugSpawnAngularVelocityMin`) (`self.PlugSpawnAngularVelocityMax`))) "None" false)
  (`KismetArrayLibrary.Array_Add` (`self.PlugsSection`) _asplug_bp))

(fn `SpawnPlugs`
  (locals (RandomNumber :type Integer))
  (bind _plugspawnarea (`self.PlugSpawnArea`))
  (bind _plugspawnarea_2 (`self.PlugSpawnArea`))
  (bind _returnvalue (`KismetArrayLibrary.Array_Length` (`self.SequecePlugs`)))
  (for _array_element (`self.SequecePlugs`)
    (bind _boxextent (`/Game/-Blueprints/-LevelPrototype/Antoine/PlugSpawnArea.GetBoxExtent` _plugspawnarea_2))
    (`self.SpawnPlug` (`KismetMathLibrary.MakeTransform` (`KismetMathLibrary.RandomPointInBoundingBox` (`self.K2_GetActorLocation` _plugspawnarea_2) _boxextent) (struct) (0.25 0.25 0.25)) _array_element))
  (bind _output_get (set `local.RandomNumber` (`KismetMathLibrary.RandomIntegerInRange` (`self.NbrPlugsToSpawnMin`) (`self.NbrPlugsToSpawnMax`))))
  (if (> _output_get _returnvalue)
    (for _ (range _returnvalue (`local.RandomNumber`))
      (bind _boxextent_2 (`/Game/-Blueprints/-LevelPrototype/Antoine/PlugSpawnArea.GetBoxExtent` _plugspawnarea))
      (`self.SpawnPlug` (`KismetMathLibrary.MakeTransform` (`KismetMathLibrary.RandomPointInBoundingBox` (`self.K2_GetActorLocation` _plugspawnarea) _boxextent_2) (struct) (0.25 0.25 0.25)) (cast `/Game/-Blueprints/-LevelPrototype/Antoine/PlugType` (`KismetMathLibrary.Conv_IntToByte` (`KismetMathLibrary.RandomIntegerInRange` 0 (- (enumcount `/Game/-Blueprints/-LevelPrototype/Antoine/PlugType`) 3))))))))

(fn `UserConstructionScript`)