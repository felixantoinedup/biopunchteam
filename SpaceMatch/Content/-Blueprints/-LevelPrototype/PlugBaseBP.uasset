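; Base Blueprint for a plug prop that robots can magnetically attract, hold and place.
; MaganeticAttract uses a timeline and VInterpTo to pull it toward the attractor's Pelvis socket with physics off, then attaches it to RightHand and notifies Robot_ChildBP.
; GrabPlug and PlacePlug manage held/placed flags and the holder, with placement clearing RobotBP's HoldingPlug.
; SetPlug only records the holder, as its attach logic is disconnected; ThrowPlug is empty.
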(event `MaganeticAttract`
  (params (ActorToAttractorTo :type "Actor Object Reference"))
  (bind _actorattractedto (`self.ActorAttractedTo`))
  (bind _location (.location (`self.GetTransform`)))
  (bind _rootcomponent (`Actor.RootComponent` _actorattractedto))
  (bind _returnvalue (`SceneComponent.GetSocketLocation` _rootcomponent "Pelvis"))
  (set `self.ActorAttractedTo` ActorToAttractorTo)
  (bind _output_get (set `self.BeingPulled` true))
  (if (and _output_get (not (== _location _returnvalue :`ErrorTolerance` 0.1)))
    (bind (_direction _newtrack_0) (`Timeline|Timeline_0` :!via `PlayFromStart`)
      (:`Update`
        (`self.K2_SetActorLocation` (+ _newtrack_0 (`KismetMathLibrary.VInterpTo` _location _returnvalue (`GameplayStatics.GetWorldDeltaSeconds`) 5.0)))
        (`PrimitiveComponent.SetSimulatePhysics` (`self.Plug`) false))
      (:`Finished`
        (set `self.BeingPulled` true)
        (bind _asrobot_child_bp (cast `/Game/-Blueprints/Robot_ChildBP` _actorattractedto))
        (`self.K2_AttachToComponent` _rootcomponent "RightHand" "KeepWorld" "KeepRelative" "KeepRelative" false)
        (`/Game/-Blueprints/Robot_ChildBP.SetObjectAttached` _asrobot_child_bp (`ActorComponent.GetOwner` (`self.Plug`)))
        (set `self.IsHolded` true)))))

(fn `GrabPlug`
  (params (NewHolder :type "Actor Object Reference") (Parent :type "SceneComponent Object Reference"))
  (if (`self.IsHolded`)
    _
    (elif (not (`self.IsPlaced`))
      (`self.SetPlug` NewHolder Parent)
      (set `self.IsHolded` true)
      (set `self.IsPlaced` false))))

(fn `PlacePlug`
  (params (NewHolder :type "Actor Object Reference") (Parent :type "SceneComponent Object Reference"))
  (if (`self.IsHolded`)
    (bind _asrobot_bp (cast `/Game/-Blueprints/RobotBP` (`self.Holder`)))
    (set `/Game/-Blueprints/RobotBP.HoldingPlug` false _asrobot_bp)
    (`self.SetPlug` NewHolder Parent)
    (set `self.IsHolded` false)
    (set `self.IsPlaced` true)))

(fn `SetPlug`
  (params (NewHolder :type "Actor Object Reference") (Parent :type "SceneComponent Object Reference"))
  (set `self.Holder` NewHolder))

(fn `ThrowPlug`)

(fn `UserConstructionScript`)