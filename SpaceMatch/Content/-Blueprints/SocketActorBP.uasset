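; Socket actor that can be magnetically pulled to the player pawn's RightHand socket and attached there.
; MaganeticAttract starts a timeline that disables mesh physics and moves the actor by VInterpTo toward the socket, adding the track value as an offset.
; When the timeline finishes, it attaches to the socket and registers the mesh's owner with Robot_ChildBP as the attached object.
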(event `self.ReceiveTick`
  (params (DeltaSeconds :type "Float (single-precision)")))

(event `MaganeticAttract`
  (bind _returnvalue (`GameplayStatics.GetPlayerPawn` 0))
  (bind _location (.location (`self.GetTransform`)))
  (bind _rootcomponent (`Actor.RootComponent` _returnvalue))
  (bind _returnvalue_2 (`SceneComponent.GetSocketLocation` _rootcomponent "RightHand"))
  (bind _output_get (set `self.BeginPulled` true))
  (if (and _output_get (not (== _location _returnvalue_2 :`ErrorTolerance` 0.1)))
    (bind (_direction _newtrack_0) (`Timeline|Timeline_0` :!via `PlayFromStart`)
      (:`Update`
        (`self.K2_SetActorLocation` (+ _newtrack_0 (`KismetMathLibrary.VInterpTo` _location _returnvalue_2 (`GameplayStatics.GetWorldDeltaSeconds`) 5.0)))
        (`PrimitiveComponent.SetSimulatePhysics` (`self.StaticMesh`) false))
      (:`Finished`
        (`self.K2_AttachToComponent` _rootcomponent "RightHand" "KeepWorld" "KeepRelative" "KeepRelative" false)
        (set `self.BeginPulled` false)
        (bind _asrobot_child_bp (cast `/Game/FlyingBP/Blueprints/Robot_ChildBP` _returnvalue))
        (`/Game/FlyingBP/Blueprints/Robot_ChildBP.SetObjectAttached` _asrobot_child_bp (`ActorComponent.GetOwner` (`self.StaticMesh`)))))))

(fn `UserConstructionScript`)