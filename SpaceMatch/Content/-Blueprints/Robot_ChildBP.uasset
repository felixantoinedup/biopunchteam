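; Robot child Blueprint that adds magnetic grabbing and releasing of plug objects on the GrabObject input.
; With nothing attached, a forward sphere trace with persistent debug drawing finds a PlugBaseBP and calls its MaganeticAttract, passing itself.
; SetObjectAttached records the held actor, so the next press detaches it.
; Release re-enables physics with gravity off and nudges the object along the robot's forward vector.
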(event `InputAction|GrabObject`
  (params (Key :type "Key Structure"))
  (:`Pressed`
    (if (`self.UsableObjAttached`)
      (`self.DetachObject`)
      (else
        (`self.RayCastGrabObject`)))))

(fn `DetachObject`
  (bind _usableobject (`self.UsableObject`))
  (if (`KismetSystemLibrary.IsValid` _usableobject)
    (`self.K2_DetachFromActor` _usableobject "KeepWorld" "KeepWorld" "KeepWorld")
    (set `self.UsableObjAttached` false)
    (bind _asprimitive_component (cast `PrimitiveComponent` (`Actor.RootComponent` _usableobject)))
    (`PrimitiveComponent.SetSimulatePhysics` _asprimitive_component true)
    (`PrimitiveComponent.SetEnableGravity` _asprimitive_component false)
    (`PrimitiveComponent.SetAllPhysicsLinearVelocity` _asprimitive_component (* (`SceneComponent.GetForwardVector` (`self.RootComponent`)) 50.0) true)))

(fn `RayCastGrabObject`
  (bind _robot (`self.Robot`))
  (bind _returnvalue (`SceneComponent.K2_GetComponentLocation` _robot))
  (bind _outhit (`KismetSystemLibrary.SphereTraceSingle` :`Start` _returnvalue :`End` (+ _returnvalue (* (`SceneComponent.GetForwardVector` _robot) 5000.0)) :`Radius` 50.0 :`TraceChannel` "TraceTypeQuery3" :`DrawDebugType` "Persistent"))
  (bind _asplug_base_bp (cast `/Game/-Blueprints/-LevelPrototype/PlugBaseBP` (`.HitActor` (`GameplayStatics.BreakHitResult` _outhit))))
  (`/Game/-Blueprints/-LevelPrototype/PlugBaseBP.MaganeticAttract` _asplug_base_bp self))

(fn `SetObjectAttached`
  (params (ActorRef :type "Actor Object Reference"))
  (set `self.UsableObjAttached` true)
  (set `self.UsableObject` ActorRef))

(fn `UserConstructionScript`
  (`parent.UserConstructionScript`))