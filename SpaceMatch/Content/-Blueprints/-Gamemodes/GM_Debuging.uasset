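; GM_Debuging is a game mode, apparently for debugging, that can run with a second local player.
; On BeginPlay it creates and spawns that player when SpawnSecondPlayer is set.
; ChoosePlayerStart counts spawns to pick the Player Start tagged Player2 for the second player and Player1 for any other.
; Without a tag match, it still returns the loop's array element.
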(event `self.ReceiveBeginPlay`
  (if (`self.SpawnSecondPlayer`)
    (`GameplayStatics.CreatePlayer` -1)))

(fn `ChoosePlayerStart`
  (params (Player :type "Controller Object Reference"))
  (returns (ReturnValue :type "Actor Object Reference"))
  (bind _result (`/Engine/EditorBlueprintResources/StandardMacros.IncrementInt` (`self.NbrPlayersSpawned`))
    (:`  `
      (switch `int` _result
        (:`Default`
          (set `self.PlayerStartName` "Player1" :!label _label))
        (:`1`
          (goto _label))
        (:`2`
          (set `self.PlayerStartName` "Player2")))
      (bind _outactors (`GameplayStatics.GetAllActorsOfClass` "/Script/Engine.PlayerStart"))
      (for _array_element _outactors
        (if (== (`PlayerStart.PlayerStartTag` _array_element) (`self.PlayerStartName`))
          (return _array_element)))
      (return _array_element))))

(fn `UserConstructionScript`)