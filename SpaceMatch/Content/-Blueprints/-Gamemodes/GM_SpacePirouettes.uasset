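; Main game mode for Space Pirouettes that sets up local multiplayer and player spawn points.
; On BeginPlay it reads the player count from the game instance, creates a second local player when needed, and applies the player 2 material to its RobotBP pawn.
; The ChoosePlayerStart override counts spawns to select the PlayerStart tagged Player1 or Player2.
; An alternative spawn-and-possess path for RobotBP_Player2 is left unconnected.
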(event `self.ReceiveBeginPlay`
  (`KismetSystemLibrary.PrintString` "Gamemode says: You are in the main game mode" true true (struct :`R` 1.0 :`G` 0.042226 :`A` 1.0))
  (bind _asspace_pirouettes_game_instance_bp (cast `/Game/-Blueprints/SpacePirouettes_GameInstanceBP` (`GameplayStatics.GetGameInstance`)))
  (if (>= (`/Game/-Blueprints/SpacePirouettes_GameInstanceBP.numberPlayers` _asspace_pirouettes_game_instance_bp) 2)
    (bind _returnvalue (`GameplayStatics.CreatePlayer` -1))
    (bind _asrobot_bp (cast `/Game/-Blueprints/RobotBP` (`Controller.K2_GetPawn` _returnvalue)))
    (`/Game/-Blueprints/RobotBP.SetMatPlayer2` _asrobot_bp)))

(fn `ChoosePlayerStart`
  (params (Player :type "Controller Object Reference"))
  (returns (ReturnValue :type "Actor Object Reference"))
  (bind _result (`/Engine/EditorBlueprintResources/StandardMacros.IncrementInt` (`self.NbrPlayersSpawned`))
    (:`  `
      (switch `int` _result
        (:`Default`
          (set `self.PlayerStartName` "Player1" :!label _label))
        (:`1`
          (goto _label))
        (:`2`
          (set `self.PlayerStartName` "Player2")))
      (bind _outactors (`GameplayStatics.GetAllActorsOfClass` "/Script/Engine.PlayerStart"))
      (for _array_element _outactors
        (if (== (`PlayerStart.PlayerStartTag` _array_element) (`self.PlayerStartName`))
          (return _array_element)))
      (return _array_element))))

(fn `UserConstructionScript`)